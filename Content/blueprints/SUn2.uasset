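; Sun actor that drives a simple day and night cycle by rotating itself.
; Each Tick it adds local pitch scaled by delta time and SunSpeed, then sets the LightSwitch flag true while actor pitch is above zero, which it treats as night, and false otherwise.
; Debug prints show the rotation, night state and flag value; nothing in these graphs reads LightSwitch beyond printing it.
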(event EventBeginPlay)

(event EventTick
  (params (DeltaSeconds :type Float%20%28single-precision%29))
  (bind _returnvalue (Transformation|GetActorRotation))
  (bind _pitch (Math|Rotator|BreakRotator _returnvalue))
  (bind _returnvalue_2 (> _pitch 0.0))
  (Development|PrintString "Hello")
  (Development|PrintString (Utilities|String|ToString(Rotator) _returnvalue))
  (Transformation|AddActorLocalRotation (Math|Rotator|MakeRotator 0.0 (* DeltaSeconds (Variables|Default|GetsunSpeed)) 0.0) false false)
  (Development|PrintString "NIGHT" _returnvalue_2)
  (if _returnvalue_2
    (bind _output_get (Variables|Default|SetlightSwitch true))
    (Development|PrintString (Utilities|String|ToString(Boolean) _output_get))
    (else
      (bind _output_get_2 (Variables|Default|SetlightSwitch false))
      (Development|PrintString (Utilities|String|ToString(Boolean) _output_get_2)))))

(event Collision|EventActorBeginOverlap
  (params (OtherActor :type Actor%20Object%20Reference)))

(fn ConstructionScript)