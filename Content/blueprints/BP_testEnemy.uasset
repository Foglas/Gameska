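; BP_testEnemy is a test enemy character that wanders the navmesh, chases pawns it sees and dies from damage.
; A Move loop walks it to random navigable points, restarting after each successful arrival.
; PawnSensing triggers a faster running chase, with a retriggerable delay that returns it to walking and wandering after sightings stop.
; TakeDamage subtracts HP with debug prints, then plays a death animation and destroys the actor after a delay.
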(event OnSeePawn(PawnSensing)
  (params (Pawn :type Pawn%20Object%20Reference))
  (Utilities|FlowControl|Sequence
    (:then_0
      (Components|Animation|PlayAnimation (Variables|Character|GetMesh) "/Game/BookHeadMonster/Demo/Animations/MM_Run_Fwd.MM_Run_Fwd" true)
      (Variables|/Script/Engine.CharacterMovementComponent|SetMaxWalkSpeed (Variables|Character|GetCharacterMovement) 5e+02))
    (:then_1
      (AI|AIMoveTo self "0, 0, 0" Pawn 5.0 false
        (:then
          (Utilities|FlowControl|RetriggerableDelay 2.0)
          (Components|Animation|PlayAnimation (Variables|Character|GetMesh) "/Game/BookHeadMonster/Demo/Animations/MM_Walk_Fwd.MM_Walk_Fwd" false)
          (Variables|/Script/Engine.CharacterMovementComponent|SetMaxWalkSpeed (Variables|Character|GetCharacterMovement) 1.3e+02)
          (CallFunction|Move))))))

(event Custom|move
  (Components|Animation|PlayAnimation (Variables|Character|GetMesh) "/Game/BookHeadMonster/Demo/Animations/BS_MM_WalkRun.BS_MM_WalkRun" false)
  (bind _randomlocation (Class|NavigationSystemV1|GetRandomLocationinNavigableRadius (Transformation|GetActorLocation) 1e+03 0 0))
  (AI|AIMoveTo self _randomlocation 0 5.0 false
    (:OnSuccess
      (CallFunction|Move))))

(event Custom|Take%20Damage
  (params (DMG :type Float%20%28double-precision%29))
  (if (> (Variables|Default|GetHP) 0.0)
    (Development|PrintString "DMG TAKEN")
    (bind _output_get (Variables|Default|SetHP (- (Variables|Default|GetHP) DMG)))
    (Development|PrintString (Utilities|String|ToString(Float) _output_get))
    (if (<= (Variables|Default|GetHP) 0.0)
      (Components|Animation|PlayAnimation (Variables|Character|GetMesh) "/Game/AnimStarterPack/UE5_ANIMATIONS/Death_1.Death_1" false)
      (Utilities|FlowControl|Delay 3.0)
      (Actor|DestroyActor))))

(event EventBeginPlay
  (CallFunction|Move))

(fn ConstructionScript)