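; BP_SpawnHandler is an actor that keeps the level populated with enemies, up to a MaxEnemies cap.
; A looping timer started on BeginPlay fires every second and counts live BP_EnemyMaster actors.
; Below the cap, it spawns a random EnemyClass entry at a random reachable navmesh point within a very large radius around itself.
; Each tick prints either the spawned enemy's name or the current count.
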(event Custom|SpawnEnemies
  (bind _outactors (Actor|GetAllActorsOfClass "/Game/blueprints/BP_EnemyMaster.BP_EnemyMaster_C"))
  (if (< (Utilities|Array|Length _outactors) (Variables|Default|Getmax%20enemies))
    (bind _returnvalue (Game|SpawnActorfromClass (Utilities|Array|Get(acopy) (Variables|Default|GetEnemyClass) (Math|Random|RandomIntegerinRange 0 (Utilities|Array|Length (Variables|Default|GetEnemyClass)))) (Math|Transform|MakeTransform (.RandomLocation (AI|Navigation|GetRandomReachablePointinRadius (Transformation|GetActorLocation) 1e+06 0 0)) "0, 0, 0" "1.000000,1.000000,1.000000") "AdjustIfPossibleButAlwaysSpawn" "OverrideRootScale" 0 0))
    (Development|PrintString (Utilities|GetDisplayName _returnvalue))
    (else
      (Development|PrintString (Utilities|String|ToString(Integer) (Utilities|Array|Length _outactors))))))

(event EventBeginPlay
  (Utilities|Time|SetTimerbyEvent (delegate Custom|SpawnEnemies) 1.0 true))

(fn ConstructionScript)