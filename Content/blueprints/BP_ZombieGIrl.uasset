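; BP_ZombieGIrl is a zombie character that wanders at random and chases pawns it sees.
; Move plays the walk animation and walks to a random navigable point nearby, repeating on success.
; PawnSensing switches it to a faster run toward the seen pawn.
; Each sighting resets a RetriggerableDelay, so it resumes walking and wandering two seconds after the last sighting.
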(event OnSeePawn(PawnSensing)
  (params (Pawn :type Pawn%20Object%20Reference))
  (Utilities|FlowControl|Sequence
    (:then_0
      (Components|Animation|PlayAnimation (Variables|Character|GetMesh) "/Game/blueprints/zombie_run.zombie_run" true)
      (Variables|/Script/Engine.CharacterMovementComponent|SetMaxWalkSpeed (Variables|Character|GetCharacterMovement) 5e+02))
    (:then_1
      (AI|AIMoveTo self "0, 0, 0" Pawn 5.0 false
        (:then
          (Utilities|FlowControl|RetriggerableDelay 2.0)
          (Components|Animation|PlayAnimation (Variables|Character|GetMesh) "/Game/blueprints/zombie_walk.zombie_walk" true)
          (Variables|/Script/Engine.CharacterMovementComponent|SetMaxWalkSpeed (Variables|Character|GetCharacterMovement) 1.3e+02)
          (CallFunction|Move))))))

(event Custom|move
  (Components|Animation|PlayAnimation (Variables|Character|GetMesh) "/Game/blueprints/zombie_walk.zombie_walk" true)
  (bind _randomlocation (Class|NavigationSystemV1|GetRandomLocationinNavigableRadius (Transformation|GetActorLocation) 1e+03 0 0))
  (AI|AIMoveTo self _randomlocation 0 5.0 false
    (:OnSuccess
      (Development|PrintString "Hello")
      (CallFunction|Move))))

(event EventBeginPlay
  (CallFunction|Move))

(fn ConstructionScript
  (|CallParentFunction))