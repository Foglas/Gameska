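; Lighthouse actor whose light sweeps around in random steps.
; On BeginPlay it sets the light to a very high intensity and starts a self-repeating MoveLight event.
; Each cycle picks a random positive yaw offset, and a timeline lerps the light's relative yaw to it, zeroing pitch and roll.
; After a short delay the event runs again, with debug prints left in.
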(event Custom|MoveLight
  (bind _lighthouselight (Variables|Default|GetLighthouseLight))
  (bind _relativerotation (Variables|/Script/Engine.SceneComponent|GetRelativeRotation _lighthouselight))
  (bind _output_get (Variables|Default|SetStart%20Rotation (.yaw _relativerotation)))
  (Development|PrintString (Utilities|String|ToString(Float) _output_get))
  (Variables|Default|SetEnd%20Rotation (+ (.yaw _relativerotation) (Math|Random|RandomFloatinRange 1e+01 4e+01)))
  (bind _alpha (Timeline|Move%20Light PlayFromStart)
    (:Update
      (Transformation|SetRelativeRotation (Variables|Default|GetLighthouseLight) (Math|Rotator|MakeRotator 0.0 0.0 (Math|Float|Lerp (Variables|Default|GetStart%20Rotation) (Variables|Default|GetEnd%20Rotation) _alpha)) false false))
    (:Finished
      (Utilities|FlowControl|Delay 1.0)
      (Development|PrintString "AGAIN")
      (CallFunction|MoveLight))))

(event EventBeginPlay
  (Rendering|Components|Light|SetIntensity (Variables|Default|GetLighthouseLight) 999999.0)
  (CallFunction|MoveLight))

(fn ConstructionScript)