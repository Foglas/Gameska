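; Spotlight Blueprint that switches itself on or off to follow the LightSwitch flag on the level's Sun actor.
; A looping timer checks the flag periodically and applies the new intensity after a random delay, so switching can be staggered.
; While the flag is on, a self-recalling Flashing event uses delays and random rolls to occasionally play a timeline that modulates intensity as a flicker.
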(event Custom|CustomEvent
  (bind _spotlight (Variables|Default|GetSpotLight))
  (if (Variables|/Game/blueprints/Sun.Sun_C|GetLightSwitch (Variables|Default|Getsun))
    (Utilities|FlowControl|Delay (Math|Random|RandomFloatinRange 0.0 6.0))
    (Rendering|Components|Light|SetIntensity _spotlight 1e+03)
    (CallFunction|Flashing)
    (else
      (Utilities|FlowControl|Delay (Math|Random|RandomFloatinRange 0.0 6.0))
      (Rendering|Components|Light|SetIntensity _spotlight 0.0))))

(event Custom|Flashing
  (if (Variables|/Game/blueprints/Sun.Sun_C|GetLightSwitch (Variables|Default|Getsun))
    (if (< (Math|Random|RandomFloatinRange 0.0 1e+01) 2.0)
      (bind _flashing_function (Timeline|Flashing%20Timer PlayFromStart)
        (:Update
          (Rendering|Components|Light|SetIntensity (Variables|Default|GetSpotLight) (* _flashing_function 3e+03)))
        (:Finished
          (Utilities|FlowControl|Delay 5.0)
          (CallFunction|Flashing)))
      (else
        (Utilities|FlowControl|Delay 5.0)
        (CallFunction|Flashing)))))

(event EventBeginPlay
  (Rendering|Components|Light|SetIntensity (Variables|Default|GetSpotLight) 0.0)
  (Utilities|Time|SetTimerbyEvent (delegate Custom|CustomEvent) 1e+01 true)
  (bind _outactors (Actor|GetAllActorsOfClass "/Game/blueprints/Sun.Sun_C"))
  (Variables|Default|Setsun (Utilities|Array|Get(acopy) _outactors)))

(fn ConstructionScript)