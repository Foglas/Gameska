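; Invisible trigger volume that plays forest background music while the BP_Nia_origin character is inside its box.
; Entering calls a play event that starts ForestMusic with a fade-in, or waits if it is already playing, then calls itself again after a delay.
; Leaving fades the music out and stops it after a delay, but nothing cancels the replay loop, which can restart the music outside.
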(event OnComponentBeginOverlap(Box)
  (params (OverlappedComponent :type Primitive%20Component%20Object%20Reference) (OtherActor :type Actor%20Object%20Reference) (OtherComp :type Primitive%20Component%20Object%20Reference) (OtherBodyIndex :type Integer) (bFromSweep :type Boolean) (SweepResult :type Hit%20Result%20Structure%20%28by%20ref%29))
  ;[0.2379 0.7249 1] BackgroundVolume
  (Utilities|Casting|CastToBP_Nia_origin OtherActor)
  (Development|PrintString "inside")
  (CallFunction|EventPlayMusic))

(event OnComponentEndOverlap(Box)
  (params (OverlappedComponent :type Primitive%20Component%20Object%20Reference) (OtherActor :type Actor%20Object%20Reference) (OtherComp :type Primitive%20Component%20Object%20Reference) (OtherBodyIndex :type Integer))
  ;[0.2379 0.7249 1] BackgroundVolume
  (Utilities|Casting|CastToBP_Nia_origin OtherActor)
  (Development|PrintString "outside")
  (Audio|Components|Audio|AdjustVolume (Variables|Default|GetForest_music) 5.0 0.0 "Linear" :!class /Script/Engine.AudioComponent)
  (Utilities|FlowControl|Delay 5.0)
  (Audio|Components|Audio|Stop (Variables|Default|GetForest_music)))

(event Custom|event_playMusic
  ;[0.2379 0.7249 1] BackgroundVolume
  (Development|PrintString "checking for music")
  (if (Audio|Components|Audio|IsPlaying (Variables|Default|GetForest_music))
    (Utilities|FlowControl|Delay 1e+01)
    (CallFunction|EventPlayMusic)
    (else
      (Audio|Components|Audio|Play (Variables|Default|GetForest_music) 0.0)
      (Audio|Components|Audio|SetVolumeMultiplier (Variables|Default|GetForest_music) 0.1 :!class /Script/Engine.AudioComponent)
      (Audio|Components|Audio|AdjustVolume (Variables|Default|GetForest_music) 1.0 5.0 "Linear" :!class /Script/Engine.AudioComponent)
      (Utilities|FlowControl|Delay 1.2e+02)
      (CallFunction|EventPlayMusic))))

(fn ConstructionScript)