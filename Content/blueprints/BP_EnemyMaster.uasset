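; BP_EnemyMaster is an enemy character that wanders, chases pawns it sees, and dies from damage.
; Move loops AI moves to random navigable points with a walk animation.
; PawnSensing triggers a faster run toward the seen pawn, with a retriggerable delay restoring slower wandering.
; TakeDamage subtracts HP, then at zero plays the death animation and destroys the actor; Attack and Patrol are empty stubs.
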(event OnSeePawn(PawnSensing)
  (params (Pawn :type Pawn%20Object%20Reference))
  (if (not (Variables|Default|Getis%20Dead))
    (Utilities|FlowControl|Sequence
      (:then_0
        (Components|Animation|PlayAnimation (Variables|Character|GetMesh) (Variables|Default|GetRun%20Animation) true)
        (Variables|/Script/Engine.CharacterMovementComponent|SetMaxWalkSpeed (Variables|Character|GetCharacterMovement) 5e+02))
      (:then_1
        (AI|AIMoveTo self "0, 0, 0" Pawn 5.0 false
          (:then
            (Utilities|FlowControl|RetriggerableDelay 2.0)
            (Components|Animation|PlayAnimation (Variables|Character|GetMesh) (Variables|Default|GetRun%20Animation) true)
            (Variables|/Script/Engine.CharacterMovementComponent|SetMaxWalkSpeed (Variables|Character|GetCharacterMovement) 1.3e+02)
            (CallFunction|Move)))))))

(event Custom|move
  (if (not (Variables|Default|Getis%20Dead))
    (Components|Animation|PlayAnimation (Variables|Character|GetMesh) (Variables|Default|GetWalk%20Animation) true)
    (bind _randomlocation (Class|NavigationSystemV1|GetRandomLocationinNavigableRadius (Transformation|GetActorLocation) 1e+03 0 0))
    (AI|AIMoveTo self _randomlocation 0 5.0 false
      (:OnSuccess
        (CallFunction|Move)))))

(event Custom|Take%20Damage
  (params (DMG :type Float%20%28double-precision%29))
  (bind _death_animation (Variables|Default|GetDeath%20Animation))
  (if (> (Variables|Default|GetHP) 0.0)
    (Development|PrintString "DMG TAKEN")
    (bind _output_get (Variables|Default|SetHP (- (Variables|Default|GetHP) DMG)))
    (Development|PrintString (Utilities|String|ToString(Float) _output_get))
    (if (<= (Variables|Default|GetHP) 0.0)
      (Components|Movement|StopMovementImmediately (Variables|Character|GetCharacterMovement))
      (Components|Animation|PlayAnimation (Variables|Character|GetMesh) _death_animation false)
      (Variables|Default|Setis%20Dead true)
      (Utilities|FlowControl|Delay (Animation|GetPlayLength _death_animation))
      (Actor|DestroyActor))))

(event EventBeginPlay
  (CallFunction|Move))

(fn ConstructionScript)

(fn Attack)

(fn Patrol)