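; BP_Fog is a Blueprint that randomly thickens or clears a local fog volume over time.
; After an initial delay, FogDistributie picks one of two timelines at even odds, lerping height fog extinction toward a random density or zero.
; Each timeline update lerps from the current extinction, and the thickening branch re-rolls its target every update.
; When either timeline finishes, the event calls itself again after a random delay.
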(event Custom|Fog%20distributie
  (bind _localfogvolume (Variables|Default|GetLocalFogVolume))
  (bind _localfogvolume_2 (Variables|Default|GetLocalFogVolume))
  (bind _heightfogextinction (Variables|/Script/Engine.LocalFogVolumeComponent|GetHeightFogExtinction _localfogvolume_2))
  (if (>= (Math|Random|RandomFloatinRange 0.0 1.0) 0.5)
    (bind _fog_change (Timeline|Timeline PlayFromStart)
      (:Update
        (Class|LocalFogVolumeComponent|SetHeightFogExtinction _localfogvolume (Math|Float|Lerp _heightfogextinction (Math|Random|RandomFloatinRange 0.01 1.0) _fog_change)))
      (:Finished
        (Utilities|FlowControl|Delay (Math|Random|RandomFloatinRange 3e+01 1.5e+02) :!label _label)
        (CallFunction|FogDistributie)))
    (else
      (bind _fog_change_2 (Timeline|Timeline_0 PlayFromStart)
        (:Update
          (Class|LocalFogVolumeComponent|SetHeightFogExtinction _localfogvolume (Math|Float|Lerp _heightfogextinction 0.0 _fog_change_2)))
        (:Finished
          (goto _label))))))

(event EventBeginPlay
  (Utilities|FlowControl|Delay 3e+01)
  (CallFunction|FogDistributie))

(fn ConstructionScript)