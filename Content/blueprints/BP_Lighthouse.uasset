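; Lighthouse actor whose light turns in intermittent, randomly sized steps.
; BeginPlay sets the light to a high intensity and starts the self-repeating MoveLight event.
; Each pass uses a timeline to lerp the light's world yaw forward by a random 30 to 60 degrees, keeping pitch and roll, then pauses briefly before the next step.
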(event Custom|MoveLight
  (bind _lighthouselight (Variables|Default|GetLighthouseLight))
  (bind _lighthouselight_2 (Variables|Default|GetLighthouseLight))
  (bind _returnvalue (Transformation|GetWorldRotation _lighthouselight_2))
  (bind _returnvalue_2 (Transformation|GetWorldRotation _lighthouselight))
  (Variables|Default|SetStart%20Rotation (.yaw _returnvalue_2))
  (Variables|Default|SetEnd%20Rotation (+ (.yaw _returnvalue_2) (Math|Random|RandomFloatinRange 3e+01 6e+01)))
  (bind _alpha (Timeline|Move%20Light PlayFromStart)
    (:Update
      (Transformation|SetWorldRotation _lighthouselight_2 (Math|Rotator|MakeRotator (.roll _returnvalue) (.pitch _returnvalue) (Math|Float|Lerp (Variables|Default|GetStart%20Rotation) (Variables|Default|GetEnd%20Rotation) _alpha)) false false))
    (:Finished
      (Utilities|FlowControl|Delay 2.0)
      (CallFunction|MoveLight))))

(event EventBeginPlay
  (Rendering|Components|Light|SetIntensity (Variables|Default|GetLighthouseLight) 9999.0)
  (CallFunction|MoveLight))

(fn ConstructionScript)