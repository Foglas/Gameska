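; BP_DoorMaster is a swinging door that responds to an Interact event and can be locked behind a key.
; When locked, it opens only if its referenced Key is marked found; otherwise it prints a locked message.
; The DoorOpen timeline lerps the mesh's world yaw a quarter turn, in a direction set by IsOpen, then flips that flag.
; The Unlock event has no effective logic.
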(event Custom|Unlock
  (params (NewParam :type Boolean))
  (if true
    _))

(event EventBeginPlay)

(event Collision|EventActorBeginOverlap
  (params (OtherActor :type Actor%20Object%20Reference)))

(event EventTick
  (params (DeltaSeconds :type Float%20%28single-precision%29)))

(event EventInteract
  (params (Character%20Picking%20Up :type BP%20Nia%20Origin%20Object%20Reference))
  (bind _sm_door (Variables|Default|GetSM_Door))
  (bind _returnvalue (Transformation|GetWorldRotation _sm_door))
  (if (Variables|Default|GetIs%20Locked)
    (if (Variables|/Game/_SurvivalSystem/props/Keys/BP_KeyMaster.BP_KeyMaster_C|GetFound (Variables|Default|GetKey))
      (bind _output_get (Variables|Default|SetStart%20Rotation (.yaw (Transformation|GetWorldRotation (Variables|Default|GetSM_Door))) :!label _label))
      (if (Variables|Default|GetIs%20Open)
        (Variables|Default|SetEnd%20Rotation (+ _output_get 9e+01))
        (bind _alpha (Timeline|Door%20Open PlayFromStart)
          (:Update
            (Transformation|SetWorldRotation (Variables|Default|GetSM_Door) (Math|Rotator|MakeRotator (.roll _returnvalue) (.pitch _returnvalue) (Math|Float|Lerp (Variables|Default|GetStart%20Rotation) (Variables|Default|GetEnd%20Rotation) _alpha)) false false))
          (:Finished
            (Variables|Default|SetIs%20Open (not (Variables|Default|GetIs%20Open)))))
        (else
          (Variables|Default|SetEnd%20Rotation (- _output_get 9e+01))
          (Timeline|Door%20Open PlayFromStart)))
      (else
        (Development|PrintString "DOOR LOCKED")))
    (else
      (goto _label))))

(fn ConstructionScript)