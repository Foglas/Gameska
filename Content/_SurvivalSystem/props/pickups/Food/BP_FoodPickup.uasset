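; BP_FoodPickup is a respawning food pickup for the survival system.
; Its Interact event adds one to the interacting character's food inventory and prints the new count.
; It then hides the pickup mesh and disables collision on it and its radius, restoring both after a random one-to-two-minute delay rather than destroying the actor.
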(event EventInteract
  (params (Character%20Picking%20Up :type BP%20Nia%20Origin%20Object%20Reference))
  (bind _output_get (Variables|/Game/blueprints/BP_Nia_origin.BP_Nia_origin_C|SetFood%20inventory Character%20Picking%20Up (+ (Variables|/Game/blueprints/BP_Nia_origin.BP_Nia_origin_C|GetFood%20inventory Character%20Picking%20Up) 1)))
  (Development|PrintString (Utilities|String|ToString(Integer) _output_get))
  (Rendering|SetVisibility (Variables|Default|GetPickup%20Object) false true)
  (Collision|SetCollisionEnabled (Variables|Default|GetPickup%20Radius) "NoCollision")
  (Collision|SetCollisionEnabled (Variables|Default|GetPickup%20Object) "NoCollision")
  (Utilities|FlowControl|Delay (Math|Random|RandomFloatinRange 6e+01 1.2e+02))
  (Rendering|SetVisibility (Variables|Default|GetPickup%20Object) true true)
  (Collision|SetCollisionEnabled (Variables|Default|GetPickup%20Radius) "QueryAndPhysics")
  (Collision|SetCollisionEnabled (Variables|Default|GetPickup%20Object) "QueryAndPhysics"))

(fn ConstructionScript
  (|CallParentFunction))