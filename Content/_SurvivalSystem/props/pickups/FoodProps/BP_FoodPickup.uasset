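; BP_FoodPickup is a respawning food pickup for the survival system.
; When a character interacts with it, it passes its HungerPoints to that character's Eat function, then hides its mesh and disables collision on both the mesh and pickup radius.
; After a random delay of 10 to 30 seconds, it restores visibility and collision on the same actor rather than destroying and respawning it.
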(event EventBeginPlay
  (|CallParentFunction) ; This node is disabled and will not be called.\nDrag off pins to build functionality.
)

(event Collision|EventActorBeginOverlap
  (params (OtherActor :type Actor%20Object%20Reference))
  (|CallParentFunction OtherActor) ; This node is disabled and will not be called.\nDrag off pins to build functionality.
)

(event EventTick
  (params (DeltaSeconds :type Float%20%28single-precision%29))
  (|CallParentFunction DeltaSeconds) ; This node is disabled and will not be called.\nDrag off pins to build functionality.
)

(event EventInteract
  (params (Character%20Picking%20Up :type BP%20Nia%20Origin%20Object%20Reference))
  (Default|Eat Character%20Picking%20Up (Variables|Default|GetHunger%20Points))
  (Rendering|SetVisibility (Variables|Default|GetPickup%20Object) false true)
  (Collision|SetCollisionEnabled (Variables|Default|GetPickup%20Radius) "NoCollision")
  (Collision|SetCollisionEnabled (Variables|Default|GetPickup%20Object) "NoCollision")
  (Utilities|FlowControl|Delay (Math|Random|RandomFloatinRange 1e+01 3e+01))
  (Rendering|SetVisibility (Variables|Default|GetPickup%20Object) true true)
  (Collision|SetCollisionEnabled (Variables|Default|GetPickup%20Radius) "QueryAndPhysics")
  (Collision|SetCollisionEnabled (Variables|Default|GetPickup%20Object) "QueryAndPhysics"))

(fn ConstructionScript
  (|CallParentFunction))